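; Dungeon end-point pad assigned to one of two characters by its Character enum, with a pentagram base and an aura.
; The construction script creates dynamic materials for both meshes, setting a red or blue base texture and aura color to match.
; Sphere overlaps show and hide the aura when the matching character enters or leaves, treating any actor that is not TPC_FireBoy as the second character.
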(event OnComponentBeginOverlap(Sphere)
  (params (OverlappedComponent :type Primitive%20Component%20Object%20Reference) (OtherActor :type Actor%20Object%20Reference) (OtherComp :type Primitive%20Component%20Object%20Reference) (OtherBodyIndex :type Integer) (bFromSweep :type Boolean) (SweepResult :type Hit%20Result%20Structure%20%28by%20ref%29))
  (Utilities|Casting|CastToTPC_FireBoy OtherActor
    (:then
      (if (Utilities|Enum|Equal(Enum) (Variables|Default|GetCharacter) "NewEnumerator0")
        (Rendering|SetVisibility (Variables|Default|GetAura) true false)))
    (:CastFailed
      (if (Utilities|Enum|Equal(Enum) (Variables|Default|GetCharacter) "NewEnumerator1")
        (Rendering|SetVisibility (Variables|Default|GetAura) true false)))))

(event OnComponentEndOverlap(Sphere)
  (params (OverlappedComponent :type Primitive%20Component%20Object%20Reference) (OtherActor :type Actor%20Object%20Reference) (OtherComp :type Primitive%20Component%20Object%20Reference) (OtherBodyIndex :type Integer))
  (Utilities|Casting|CastToTPC_FireBoy OtherActor
    (:then
      (if (Utilities|Enum|Equal(Enum) (Variables|Default|GetCharacter) "NewEnumerator0")
        (Rendering|SetVisibility (Variables|Default|GetAura) false false)))
    (:CastFailed
      (if (Utilities|Enum|Equal(Enum) (Variables|Default|GetCharacter) "NewEnumerator1")
        (Rendering|SetVisibility (Variables|Default|GetAura) false false)))))

(event EventBeginPlay)

(event Collision|EventActorBeginOverlap
  (params (OtherActor :type Actor%20Object%20Reference)))

(event EventTick
  (params (DeltaSeconds :type Float%20%28single-precision%29)))

(fn ConstructionScript
  (bind _returnvalue (Rendering|Material|CreateDynamicMaterialInstance "/Game/Dungeon/Materials/Aura_MasterMat.Aura_MasterMat" :!class /Script/Engine.KismetMaterialLibrary))
  (Rendering|Material|SetMaterial (Variables|Default|GetAura) 0 _returnvalue)
  (Variables|Default|SetInstMatAura _returnvalue)
  (bind _returnvalue_2 (Rendering|Material|CreateDynamicMaterialInstance "/Game/POLDungeon100/Materials/DungeonPack_MasterMat.DungeonPack_MasterMat" :!class /Script/Engine.KismetMaterialLibrary))
  (Rendering|Material|SetMaterial (Variables|Default|GetSM_Env_Tiles_Pentagram_01) 0 _returnvalue_2)
  (bind _output_get (Variables|Default|SetInstMatBase _returnvalue_2))
  (if (Utilities|Enum|Equal(Enum) (Variables|Default|GetCharacter) "NewEnumerator0")
    (Rendering|Material|SetTextureParameterValue _output_get "TexParam" "/Game/POLDungeon100/Textures/DungeonPack_Texture.DungeonPack_Texture")
    (Rendering|Material|SetVectorParameterValue (Variables|Default|GetInstMatAura) "Color" "(R=0.536458,G=0.078199,B=0.000000,A=1.000000)" :!class /Script/Engine.MaterialInstanceDynamic)
    (else
      (Rendering|Material|SetTextureParameterValue _output_get "TexParam" "/Game/POLDungeon100/Textures/DungeonPackBlue_Texture.DungeonPackBlue_Texture")
      (Rendering|Material|SetVectorParameterValue (Variables|Default|GetInstMatAura) "Color" "(R=0.000000,G=0.242468,B=0.536458,A=1.000000)" :!class /Script/Engine.MaterialInstanceDynamic))))